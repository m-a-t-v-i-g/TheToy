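; BP_HUDMain is the player's main HUD, switching from the in-game HUD to the game over screen when the match ends.
; On BeginPlay it shows WBP_HUD in game-only input and binds to TheToyGameState's game timer end delegate.
; OnGameEnd replaces that widget with WBP_GameOverScreen, initialized with the game result, then enables UI-only input and the mouse cursor.
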(event `self.ReceiveBeginPlay`
  (bind _asbp_player_controller_main (cast `/Game/TheToy/Player/BP_PlayerControllerMain` (`self.GetOwningPlayerController`)))
  (bind _returnvalue (`|CreateWidget` "/Game/TheToy/UI/Widgets/WBP_HUD.WBP_HUD_C" _asbp_player_controller_main))
  (bind _output_get (set `self.HUD` _returnvalue))
  (`UserWidget.AddToViewport` _output_get 0)
  (`WidgetBlueprintLibrary.SetInputMode_GameOnly` _asbp_player_controller_main)
  (bind _asthe_toy_game_state (cast `TheToyGameState` (`GameplayStatics.GetGameState`)))
  (add `TheToyGameState.GameTimerEndDelegate` _asthe_toy_game_state (`|CreateDelegate` :!event `OnGameEnd`)))

(event `OnGameEnd`
  (params (`Game Result` :type "TheToyGameResult Structure"))
  (bind _returnvalue (`self.GetOwningPlayerController`))
  (`Widget.RemoveFromParent` (`self.HUD`))
  (bind _returnvalue_2 (`|CreateWidget` "/Game/TheToy/UI/Widgets/Game/WBP_GameOverScreen.WBP_GameOverScreen_C" _returnvalue))
  (bind _output_get (set `self.GameOverWidget` _returnvalue_2))
  (`/Game/TheToy/UI/Widgets/Game/WBP_GameOverScreen.Init Game Over Screen` _output_get `Game Result`)
  (`UserWidget.AddToViewport` _output_get 0)
  (`WidgetBlueprintLibrary.SetInputMode_UIOnlyEx` _returnvalue _output_get)
  (set `PlayerController.bShowMouseCursor` true _returnvalue))

(fn `UserConstructionScript`)